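; GA_Blink is a gameplay ability that teleports the player to a targeted point within a limited range.
; While awaiting user-confirmed target data, it replays a levitation montage, ending the ability if that montage is interrupted.
; On confirmation it commits the ability, disables movement and plays a revelation montage.
; A montage trigger gameplay event performs the teleport and restores walking; montage completion or interruption also restores walking and ends the ability.
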(event Custom|LoopAnimation
  (|PlayMontageandWaitProxy "None" "/Game/Animations/CombatMagicAnims/Animations/AS_Levitating_Montage.AS_Levitating_Montage" 1.0 "None" true 1.0 0.0 false
    (:OnBlendOut
      (if (Variables|Default|GetWaitingDataTarget)
        (CallFunction|LoopAnimation)))
    (:OnInterrupted
      (if (Variables|Default|GetWaitingDataTarget)
        (Ability|EndAbility)))))

(event Custom|ComfimTeleport
  (bind _returnvalue (Game|GetPlayerCharacter 0))
  (bind _asbp_player (Utilities|Casting|CastToBP_Player _returnvalue))
  (bind _charactermovement (Variables|/Script/Engine.Character|GetCharacterMovement _asbp_player))
  (bind _returnvalue_2 (Ability|CommitAbility))
  (if _returnvalue_2
    (Pawn|Components|CharacterMovement|DisableMovement _charactermovement)
    (|PlayMontageandWaitProxy "None" "/Game/Animations/CombatMagicAnims/Animations/AS_Revelation_Montage.AS_Revelation_Montage" 1.0 "None" true 1.0 0.0 false
      (:then
        (Ability|Tasks|WaitGameplayEvent "(TagName=\"Event.Montage.Trigger\")" 0
          (:EventReceived
            (Pawn|Components|CharacterMovement|SetMovementMode _charactermovement "MOVE_Walking" 0)
            (Transformation|SetActorRelativeLocation (.AsBP%20Player (Utilities|Casting|CastToBP_Player (Game|GetPlayerCharacter 0))) (Variables|Default|GetTeleportLocation) false true))))
      (:OnCompleted
        (Ability|EndAbility :!label _label)
        (Pawn|Components|CharacterMovement|SetMovementMode _charactermovement "MOVE_Walking" 0))
      (:OnInterrupted
        (goto _label)))
    (else
      (Ability|EndAbility))))

(event Ability|EventActivateAbility
  (CallFunction|LoopAnimation)
  (Variables|Default|SetWaitingDataTarget true)
  (bind _data (|WaitTargetData :ConfirmationType "UserConfirmed" :Class "/Game/GAS/TargetingActors/GATargetActor_GroundTrace_Decal.GATargetActor_GroundTrace_Decal_C" :MaxRange 1.2e+03 :TraceProfile "(Name=\"NoCollision\")" :StartLocation (Class|GameplayAbility|MakeTargetLocationInfofromOwnerActor) :ReticleClass 0)
    (:ValidData
      (Variables|Default|SetTeleportLocation (.Location (Collision|BreakHitResult (Ability|TargetData|GetHitResultfromTargetData _data))))
      (Variables|Default|SetWaitingDataTarget false)
      (CallFunction|ComfimTeleport))))