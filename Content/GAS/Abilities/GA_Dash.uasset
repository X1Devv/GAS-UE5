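; Gameplay ability that makes the avatar dash through a short constant-force root motion task.
; Direction follows the pawn's last movement input, falling back to actor forward when there is none.
; Cost commits on activation and a dash gameplay cue plays until the ability ends.
; When the force finishes, velocity is clamped to movement max speed, then cooldown commits and the ability ends.
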(event Ability|EventActivateAbility
  (Ability|CommitAbilityCost false)
  (Ability|Tasks|ApplyRootMotionConstantForce "None" (CallFunction|GetDashDiraction) 1e+03 0.3 false 0 "ClampVelocity" "0, 0, 0" (CallFunction|GetMaxSpeed)
    (:then
      (GameplayCue|AddGameplayCue :GameplayCueTag "(TagName=\"GameplayCue.Dash.Active\")"))
    (:OnFinish
      (Ability|CommitAbilityCooldown false)
      (Ability|EndAbility))))

(fn GetDashDiraction
  (bind _aspawn (Utilities|Casting|CastToPawn (Ability|GetAvatarActorfromActorInfo))
    (:then
      (if (Math|Vector|VectorIsZero (Class|Pawn|GetLastMovementInputVector _aspawn))
        _
        (else
          (return (Class|Pawn|GetLastMovementInputVector _aspawn)))))
    (:CastFailed
      _))
  (return (Transformation|GetActorForwardVector (Ability|GetAvatarActorfromActorInfo))))

(fn GetMaxSpeed
  (bind _aspawn (Utilities|Casting|CastToPawn (Ability|GetAvatarActorfromActorInfo))
    (:then
      (return (Class|MovementComponent|GetMaxSpeed (Pawn|GetMovementComponent _aspawn))))
    (:CastFailed
      ;[0.15 0.15 0.15 0.5] bad implementation. I'll fix it in the next update.
      (return 5e+02))))