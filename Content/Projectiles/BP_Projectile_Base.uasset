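; Base projectile Blueprint that flies toward a target location and delivers a Gameplay Ability System effect to the actor it overlaps.
; On BeginPlay it aims its movement at the target using Speed and fires a spawn gameplay cue.
; Overlapping a non-instigator applies the effect spec on authority if an ability system component exists, then destroys the projectile.
; Blocking hits also destroy it, and destruction fires the impact cue.
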(event OnComponentBeginOverlap(Sphere)
  (params (OverlappedComponent :type Primitive%20Component%20Object%20Reference) (OtherActor :type Actor%20Object%20Reference) (OtherComp :type Primitive%20Component%20Object%20Reference) (OtherBodyIndex :type Integer) (bFromSweep :type Boolean) (SweepResult :type Hit%20Result%20Structure%20%28by%20ref%29))
  (bind _returnvalue (Ability|GetAbilitySystemComponent OtherActor))
  (if (!= OtherActor (Variables|Actor|GetInstigator))
    (Utilities|IsValid _returnvalue
      (:Is%20Valid
        (Networking|SwitchHasAuthority
          (:Authority
            (GameplayEffects|ApplyGameplayEffectSpecToSelf _returnvalue (Variables|GameplayEffect|GetEffectSpecHandle)))
          (:Remote
            _)))
      (:Is%20Not%20Valid
        _))
    (Actor|DestroyActor)))

(event OnComponentHit(Sphere)
  (params (HitComponent :type Primitive%20Component%20Object%20Reference) (OtherActor :type Actor%20Object%20Reference) (OtherComp :type Primitive%20Component%20Object%20Reference) (NormalImpulse :type Vector :default "0, 0, 0") (Hit :type Hit%20Result%20Structure%20%28by%20ref%29))
  (Actor|DestroyActor))

(event EventBeginPlay
  (bind _projectilemovement (Variables|Default|GetProjectileMovement))
  (Variables|/Script/Engine.MovementComponent|SetVelocity _projectilemovement (* (Math|Vector|GetUnitDirection(Vector) (Transformation|GetActorLocation) (Variables|ProjectileSettings|GetTargetLocation)) (Variables|ProjectileSettings|GetSpeed)))
  (Components|Activation|Activate _projectilemovement false)
  (GameplayCue|ExecuteGameplayCueOnActor(Burst) self (Variables|GameplayCue|GetGameplay%20Cue%20Spawn) (Ability|GameplayCue|MakeGameplayCueParameters :Location (Transformation|GetActorLocation))))

(event EventDestroyed
  (GameplayCue|ExecuteGameplayCueOnActor(Burst) self (Variables|GameplayCue|GetGameplay%20Cue%20Impact) (Ability|GameplayCue|MakeGameplayCueParameters :Location (Transformation|GetActorLocation))))

(fn ConstructionScript)